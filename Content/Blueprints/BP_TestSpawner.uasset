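; BP_TestSpawner is a test enemy spawner that feeds an encounter's objective.
; On BeginPlay it binds SpawnEnemies to the owning encounter's start-begin event.
; SpawnEnemies creates a small batch of BP_TestEnemy at random X/Y points in the SpawnArea box, using its relative location and a fixed height, and registers itself as their spawner.
; Its EnemyDied event reports objective success to the encounter through UpdateObjectiveSucceed.
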(event Custom|Spawn%20Enemies
  (params (Encounter :type Encounter%20Object%20Reference))
  (bind _spawnarea (Variables|Default|GetSpawnArea))
  (bind _relativelocation (Variables|/Script/Engine.SceneComponent|GetRelativeLocation _spawnarea))
  (bind _boxextent (Variables|/Script/Engine.BoxComponent|GetBoxExtent _spawnarea))
  (bind _returnvalue (Math|Random|RandomPointinBoundingBox _relativelocation _boxextent))
  (bind (_x _y) (Class|KismetMathLibrary|BreakVector3f _returnvalue))
  (for _index (range 0 2)
    (bind _returnvalue_2 (Game|SpawnActorfromClass "/Game/Blueprints/BP_TestEnemy.BP_TestEnemy_C" (Math|Conversions|ToTransform(Vector) (Math|Vector|MakeVector _x _y 7e+01)) "Undefined" 0 0))
    (Default|SetOwningSpawner _returnvalue_2 self)))

(event Custom|EnemyDied
  (Class|Encounter|UpdateObjectiveSucceed (Variables|Default|GetOwningEncounter)))

(event EventBeginPlay
  (EventDispatchers|BindEventtoEncounteronStartBegin (Variables|Default|GetOwningEncounter) (delegate Custom|Spawn%20Enemies)))

(fn ConstructionScript)