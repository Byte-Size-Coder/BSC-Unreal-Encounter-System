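; BP_TestDialog is a test Blueprint that shows dialog messages when encounters in the level begin or are won.
; On BeginPlay it binds to the intro-begin and succeed-begin events of every encounter in the level.
; Each event calls OpenDialog, which creates a BPW_TestDialog widget and passes it the encounter, text and itself.
; CloseDialog removes and clears the stored widget, while RegisterEncounters is an empty stub.
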(event Custom|WonEncounter
  (params (Encounter :type Encounter%20Object%20Reference))
  (CallFunction|OpenDialog Encounter "You have succeeded the encounter!"))

(event Custom|EncounterOnIntroBegin_Event
  (params (Encounter :type Encounter%20Object%20Reference))
  (CallFunction|OpenDialog Encounter "Encounter Has Begun! Destroy all Ene mies"))

(event EventBeginPlay
  (bind _encounters (CallFunction|GetAllEncountersinLevel))
  (for _array_element _encounters
    (EventDispatchers|AssignEncounteronIntroBegin _array_element (delegate Custom|EncounterOnIntroBegin_Event))
    (EventDispatchers|BindEventtoEncounteronSucceedBegin _array_element (delegate Custom|WonEncounter))))

(event Collision|EventActorBeginOverlap
  (params (OtherActor :type Actor%20Object%20Reference)))

(event EventTick
  (params (DeltaSeconds :type Float%20%28single-precision%29)))

(fn ConstructionScript)

(fn RegisterEncounters)

(fn OpenDialog
  (params (Encounter :type Encounter%20Object%20Reference) (Text :type String))
  (bind _returnvalue (UserInterface|CreateWidget "/Game/Blueprints/BPW_TestDialog.BPW_TestDialog_C"))
  (bind _output_get (Variables|Default|SetDialogWidget _returnvalue))
  (UserInterface|Viewport|AddtoViewport _output_get 0)
  (Default|OpenConversation _output_get Encounter Text self))

(fn CloseDialog
  (Widget|RemovefromParent (Variables|Default|GetDialogWidget))
  (Variables|Default|SetDialogWidget 0))